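; BP_ExteriorDoor is an exterior door that opens and closes instantly through trigger boxes.
; Beginning an overlap with Box_Enter sets the Arrow component's relative rotation to OpenRotation, and ending an overlap with Box_Exit sets it to Closedrotation.
; Both events print debug strings and check for the Player tag, but the check does not gate the rotation, so any overlapping actor triggers it.
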(event OnComponentBeginOverlap(Box_Enter)
  (params (OverlappedComponent :type Primitive%20Component%20Object%20Reference) (OtherActor :type Actor%20Object%20Reference) (OtherComp :type Primitive%20Component%20Object%20Reference) (OtherBodyIndex :type Integer) (bFromSweep :type Boolean) (SweepResult :type Hit%20Result%20Structure%20%28by%20ref%29))
  (Development|PrintString "Hello")
  (if (Actor|ActorHasTag OtherActor "Player")
    _
    (else
      _))
  (Transformation|SetRelativeRotation (Variables|Default|GetArrow) (Variables|Default|GetOpenRotation) false false))

(event OnComponentEndOverlap(Box_Exit)
  (params (OverlappedComponent :type Primitive%20Component%20Object%20Reference) (OtherActor :type Actor%20Object%20Reference) (OtherComp :type Primitive%20Component%20Object%20Reference) (OtherBodyIndex :type Integer))
  (Development|PrintString "Hello2")
  (if (Actor|ActorHasTag OtherActor "Player")
    _
    (else
      _))
  (Transformation|SetRelativeRotation (Variables|Default|GetArrow) (Variables|Default|GetClosedrotation) false false))

(fn ConstructionScript)