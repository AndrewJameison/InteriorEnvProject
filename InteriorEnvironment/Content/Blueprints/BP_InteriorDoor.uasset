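; Interior door Blueprint that swings open and closed through two trigger volumes, apparently for the scientist's chambers.
; OpenBox overlap plays the Open timeline and RoomBox overlap plays Close, each driving the Arrow component's yaw from its DoorRotation track.
; Both branches of each Player tag check play the timeline, so any overlapping actor triggers it.
; Debug prints remain, and the commented lock and alarm are not implemented here.
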(event OnComponentBeginOverlap(OpenBox)
  (params (OverlappedComponent :type Primitive%20Component%20Object%20Reference) (OtherActor :type Actor%20Object%20Reference) (OtherComp :type Primitive%20Component%20Object%20Reference) (OtherBodyIndex :type Integer) (bFromSweep :type Boolean) (SweepResult :type Hit%20Result%20Structure%20%28by%20ref%29))
  (Development|PrintString "Hello")
  (if (Actor|ActorHasTag OtherActor "Player")
    (bind _door_rotation (Timeline|Open PlayFromStart)
      (:Update
        (Transformation|SetRelativeRotation (Variables|Default|GetArrow) (Math|Rotator|MakeRotator 0.0 0.0 _door_rotation) false false)))
    (else
      (Timeline|Open PlayFromStart))))

(event OnComponentBeginOverlap(RoomBox)
  (params (OverlappedComponent :type Primitive%20Component%20Object%20Reference) (OtherActor :type Actor%20Object%20Reference) (OtherComp :type Primitive%20Component%20Object%20Reference) (OtherBodyIndex :type Integer) (bFromSweep :type Boolean) (SweepResult :type Hit%20Result%20Structure%20%28by%20ref%29))
  ;[0.15 0.15 0.15 0.5] The player has entered the scientist's chambers, the door locks behind them and a red alarm starts beeping near the door
  (Development|PrintString "Hello2")
  (if (Actor|ActorHasTag OtherActor "Player")
    (bind _door_rotation (Timeline|Close PlayFromStart)
      (:Update
        (Transformation|SetRelativeRotation (Variables|Default|GetArrow) (Math|Rotator|MakeRotator 0.0 0.0 _door_rotation) false false)))
    (else
      (Timeline|Close PlayFromStart))))

(fn ConstructionScript)